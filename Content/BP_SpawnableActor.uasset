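; BP_SpawnableActor is a placeable actor that shows placement feedback through the material on its static mesh.
; Each Tick, it applies the valid or invalid placement material while IsBeingPlaced is set, based on PlacementValid, and MaterialRef otherwise.
; UpdateMesh stores the given mesh reference and passes it to the SE_UpdateMesh event, which sets it on the StaticMesh component.
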(event `self.ReceiveTick`
  (params (DeltaSeconds :type "Float (single-precision)"))
  (if (`self.isBeingPlaced`)
    (if (`self.placementValid`)
      (`PrimitiveComponent.SetMaterial` (`self.StaticMesh`) 0 "/Game/Materials/MAT_Interactable_Placement_Valid.MAT_Interactable_Placement_Valid")
      (else
        (`PrimitiveComponent.SetMaterial` (`self.StaticMesh`) 0 "/Game/Materials/MAT_Interactable_Placement_Invalid.MAT_Interactable_Placement_Invalid")))
    (else
      (`PrimitiveComponent.SetMaterial` (`self.StaticMesh`) 0 (`self.materialRef`)))))

(event `SE_UpdateMesh`
  (params (mesRef :type "StaticMesh Object Reference"))
  (`StaticMeshComponent.SetStaticMesh` (`self.StaticMesh`) mesRef))

(event `UpdateMesh`
  (params (meshRef :type "StaticMesh Object Reference"))
  (bind _output_get (set `self.meshRef` meshRef))
  (`self.SE_UpdateMesh` _output_get))

(fn `UserConstructionScript`)