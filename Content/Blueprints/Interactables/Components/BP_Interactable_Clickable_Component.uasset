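; Actor component that makes its owner hoverable by the mouse cursor, apparently as an interactable object.
; On BeginPlay it binds the owner's cursor-over events, which toggle custom depth on its static meshes for highlighting and set or clear HoveredActor on BP_FirstPersonCharacter.
; InPlacementMode destroys the component, and OutOfPlacementMode adds one to the placed actor.
; Single and multiple selection events are empty, with their material-swapping logic left disconnected.
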(event `self.ReceiveBeginPlay`
  (bind _returnvalue (`self.GetOwner`))
  (bind _returnvalue_2 (`self.GetOwner`))
  (`/Engine/EditorBlueprintResources/StandardMacros.IsValid` _returnvalue
    (:`Is Valid`
      (set `self.selfOwner` _returnvalue)
      (bind _asbp_first_person_character (cast `/Game/FirstPerson/Blueprints/BP_FirstPersonCharacter` (`GameplayStatics.GetPlayerCharacter` 0)))
      (set `self.AS_BP_Char` _asbp_first_person_character)
      (set `self.staticMeshRef` (`Actor.K2_GetComponentsByClass` _returnvalue_2 "/Script/Engine.StaticMeshComponent"))
      ;[1 1 1] Highlighting of parent Actor when mouse hovers over
      (add `Actor.OnBeginCursorOver` _returnvalue_2 (delegate `OnMouseHover`))
      (add `Actor.OnEndCursorOver` _returnvalue_2 (delegate `OnMouseHoverEnd`)))))

(event `OnMouseHover`
  (params (TouchedActor :type "Actor Object Reference"))
  ;[1 1 1] Highlighting of parent Actor when mouse hovers over
  (for _array_element (`self.staticMeshRef`)
    (`PrimitiveComponent.SetRenderCustomDepth` _array_element true))
  (set `/Game/FirstPerson/Blueprints/BP_FirstPersonCharacter.hoveredActor` TouchedActor (`self.AS_BP_Char`))
  (set `self.isHovered` true))

(event `OnMouseHoverEnd`
  (params (TouchedActor :type "Actor Object Reference"))
  ;[1 1 1] Highlighting of parent Actor when mouse hovers over
  (for _array_element (`self.staticMeshRef`)
    (`PrimitiveComponent.SetRenderCustomDepth` _array_element false))
  (set `/Game/FirstPerson/Blueprints/BP_FirstPersonCharacter.hoveredActor` null (`self.AS_BP_Char`))
  (set `self.isHovered` false))

(event `OnSelectSingle`
  ;[1 1 1] Select Actor on left click
)

(event `OnSelectMultiple`
  ;[1 1 1] If already selected, deselect. Otherwise: add to resp. array. Update materials accordingly.
)

(event `InPlacementMode`
  (`self.K2_DestroyComponent`))

(event `OutOfPlacementMode`
  (params (placedActorRef :type "Actor Object Reference"))
  (`|AddComponentByClass` placedActorRef "BP_Interactable_Clickable_Component_C"))