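; Actor component for interactable fixtures that adds a light to its owning actor at runtime, based on a fixture type.
; SE_TypeOfLight passes the type to SetLightComponent, which creates a point or red-tinted spot light above the owner's static mesh, attached to it and set to replicate.
; Rect and directional light branches exist but are unconnected, and the light's OnRep function is empty.
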(event `SE_TypeOfLight`
  (params (typeOfFixture :type "/Game/ENUM_TypeOfLight Enum" :default "NewEnumerator0"))
  (`self.SetLightComponent` typeOfFixture))

(fn `OnRep_LightComponent`)

(fn `SetLightComponent`
  (params (typeOfFixture :type "/Game/ENUM_TypeOfLight Enum" :default "NewEnumerator0"))
  (bind _returnvalue (`self.GetOwner`))
  (bind _returnvalue_2 (`Actor.GetComponentByClass` _returnvalue "/Script/Engine.StaticMeshComponent"))
  (switch `/Game/ENUM_TypeOfLight` typeOfFixture
    (:`NewEnumerator0`
      (bind _returnvalue_3 (`|AddComponentByClass` _returnvalue "/Script/Engine.PointLightComponent" false (`KismetMathLibrary.MakeTransform` (0.0 0.0 150.0))))
      (`SceneComponent.K2_AttachToComponent` _returnvalue_3 _returnvalue_2 "None" "KeepRelative" "KeepRelative" "KeepRelative" true)
      (`self.SetIsReplicated` _returnvalue_3 true))
    (:`NewEnumerator1`
      (bind _returnvalue_4 (`|AddComponentByClass` _returnvalue "/Script/Engine.SpotLightComponent" false (`KismetMathLibrary.MakeTransform` (0.0 0.0 150.0))))
      (`SceneComponent.K2_AttachToComponent` _returnvalue_4 _returnvalue_2 "None" "KeepRelative" "KeepRelative" "KeepRelative" true)
      (`LightComponent.SetLightColor` _returnvalue_4 (struct :`R` 1.0 :`G` 0.009502 :`A` 1.0) true)
      (`self.SetIsReplicated` _returnvalue_4 true))))